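; Game mode for Farm Hunt that spawns the player's selected character when play begins.
; BeginPlay calls Multicast, which switches on the game instance's CharSelect, spawns Farmer Joe or Butcher Billy at the first PlayerStart found, has player controller 0 possess it, then destroys itself.
; Medic Mary and Lumber Jack only print placeholders.
; The spawn-request events are empty or uncalled, and a per-player PlayerStart assignment sits unwired.
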(event Custom|ClientRequestSpawn
  (CallFunction|ServerRequestSpawn))

(event Custom|ServerRequestSpawn)

(event Custom|Multicast
  (bind _returnvalue (Game|GetPlayerController 0))
  (bind _returnvalue_2 (Game|GetPlayerController 0))
  (bind _asmy_game_instance (Utilities|Casting|CastToMyGameInstance (Game|GetGameInstance)))
  (switch Utilities|FlowControl|Switch|SwitchonCharSelector (Variables|/Game/MyGame/MyGameBlueprints/MyGameInstance/MyGameInstance.MyGameInstance_C|GetCharSelect _asmy_game_instance)
    (:NewEnumerator19
      (Development|PrintString "No Character Chosen..."))
    (:NewEnumerator13
      (bind _outactors (Actor|GetAllActorsOfClass "/Script/Engine.PlayerStart"))
      (bind _returnvalue_3 (Game|SpawnActorfromClass "/Game/PixelCharacters/PixelFarmHunt/Pixel_Farmer.Pixel_Farmer_C" (Transformation|GetWorldTransform (Variables|/Script/Engine.Actor|GetRootComponent (Utilities|Array|Get(acopy) _outactors))) "AlwaysSpawn" _returnvalue_2 0))
      (Pawn|UnPossess _returnvalue_2)
      (Pawn|Possess _returnvalue_2 _returnvalue_3)
      (Actor|DestroyActor))
    (:NewEnumerator14
      (bind _outactors_2 (Actor|GetAllActorsOfClass "/Script/Engine.PlayerStart"))
      (bind _returnvalue_4 (Game|SpawnActorfromClass "/Game/PixelCharacters/PixelFarmHunt/Pixel_Butcher.Pixel_Butcher_C" (Transformation|GetWorldTransform (Variables|/Script/Engine.Actor|GetRootComponent (Utilities|Array|Get(acopy) _outactors_2))) "AlwaysSpawn" _returnvalue 0))
      (Pawn|UnPossess _returnvalue)
      (Pawn|Possess _returnvalue _returnvalue_4)
      (Actor|DestroyActor))
    (:NewEnumerator15
      (Development|PrintString "Medic"))
    (:NewEnumerator16
      (Development|PrintString "Lumber"))))

(event EventBeginPlay
  (CallFunction|Multicast))

(event EventTick
  (params (DeltaSeconds :type Float%20%28single-precision%29)))

(event EventPostLogin
  (params (NewPlayer :type Player%20Controller%20Object%20Reference)))

(fn ConstructionScript)