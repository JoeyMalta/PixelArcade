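; Base pickup item for the inventory system, with configurable mesh and interaction sphere, and placeholder Use, Equip and Dismantle actions.
; On local player overlap, skipped on dedicated servers, it either adds itself instantly or claims the inventory's ItemInRange slot and shows a hold-key prompt.
; Holding Interact drives a timer-polled progress bar until pickup.
; Overlapping items poll on a looping timer to claim the slot once it clears.
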(event Custom|Clear%20Interaction%20UI
  ;[1 1 1] player leaves item
  (if (== (stale Collision|EventActorEndOverlap OtherActor) (Game|GetPlayerCharacter 0))
    (Variables|/Game/StarterInventory/Blueprints/Inventory.Inventory_C|SetItem%20in%20Range (Variables|Default|GetInventory%20ref) 0) ; Clear the object if the player leaves
    (CallFunction|RemoveInteractionUI)
    (Utilities|Time|ClearandInvalidateTimerbyHandle (Variables|Internal|GetOverlapCheck%20Timer))
    (Utilities|Time|ClearandInvalidateTimerbyHandle (Variables|Internal|GetInteraction%20Timer))))

(event EventBeginPlay
  ;[1 1 1] Set player reference and Inventory reference
  (CallFunction|SetInventoryReffromPlayer))

(event Collision|EventActorBeginOverlap
  (params (OtherActor :type Actor%20Object%20Reference))
  (bind _inventory_ref (Variables|Default|GetInventory%20ref))
  ;[1 1 1] Player overlaps item
  (if (not (Networking|IsDedicatedServer)) ; do not procedd on dedicated server
    (if (== OtherActor (Game|GetPlayerCharacter 0))
      (CallFunction|SetInventoryReffromPlayer)
      (if (<= (Variables|Default|GetPickupTime) 0.0) ; If Pickup Time is 0 or less pickup instantly on touch
        (Default|AddItemtoInventory _inventory_ref self 1)
        (else
          (Utilities|IsValid (Variables|/Game/StarterInventory/Blueprints/Inventory.Inventory_C|GetItem%20in%20Range _inventory_ref)
            (:Is%20Valid
              (bind _returnvalue (Utilities|Time|SetTimerbyFunctionName 0 "Check if item overlap is cleared" 0.1 true))
              (Variables|Internal|SetOverlapCheck%20Timer _returnvalue))
            (:Is%20Not%20Valid
              (Variables|/Game/StarterInventory/Blueprints/Inventory.Inventory_C|SetItem%20in%20Range _inventory_ref self) ; this is the object that will be getting picked up
              (Utilities|IsValid (Variables|Internal|GetMessage%20Overlay%20Widget)
                (:Is%20Valid
                  (CallFunction|RemoveInteractionUI))
                (:Is%20Not%20Valid
                  _))
              (CallFunction|CreateInteractionUI (Utilities|Text|ToText(String) (Variables|Default|GetItem%20Name)) (Variables|Default|GetInteraction%20verb))
              ;[1 1 1] if the button is already being held, just strat the interaction
              (if (Variables|/Game/StarterInventory/Blueprints/Inventory.Inventory_C|GetInteraction%20Button%20Pressed (Variables|/Game/StarterInventory/FirstPerson/Blueprints/FirstPersonCharacter.FirstPersonCharacter_C|GetInventory%20Component (Variables|Internal|GetChar%20Ref)))
                (CallFunction|Interact)))))))))

(event Collision|EventActorEndOverlap
  (params (OtherActor :type Actor%20Object%20Reference))
  ;[1 1 1] player leaves item
  (if (not (Networking|IsDedicatedServer)) ; do not procedd on dedicated server
    (if (== OtherActor (Game|GetPlayerCharacter 0))
      (Variables|/Game/StarterInventory/Blueprints/Inventory.Inventory_C|SetItem%20in%20Range (Variables|Default|GetInventory%20ref) 0) ; Clear the object if the player leaves
      (CallFunction|RemoveInteractionUI)
      (Utilities|Time|ClearandInvalidateTimerbyHandle (Variables|Internal|GetOverlapCheck%20Timer))
      (Utilities|Time|ClearandInvalidateTimerbyHandle (Variables|Internal|GetInteraction%20Timer)))))

(fn ConstructionScript
  (bind _interaction_distance_scale (Variables|Default|GetInteraction%20Distance%20Scale))
  (bind _meshscale (Variables|Default|GetMeshScale))
  (bind _interaction_sphere (Variables|Default|GetInteraction%20Sphere))
  (Components|StaticMesh|SetStaticMesh (Variables|Default|GetStaticMesh) (Variables|Default|GetModel))
  (Transformation|SetRelativeScale3D (Variables|Default|GetStaticMesh) (Math|Vector|MakeVector _meshscale _meshscale _meshscale))
  (Transformation|SetRelativeScale3D _interaction_sphere (Math|Vector|MakeVector _interaction_distance_scale _interaction_distance_scale _interaction_distance_scale))
  (Rendering|SetVisibility _interaction_sphere (Variables|Default|GetShow%20Interaction%20Range) false))

(fn Interact
  (bind _message_overlay_widget (Variables|Internal|GetMessage%20Overlay%20Widget))
  (bind _progressbar_center (Variables|/Game/StarterInventory/UMG/Message_Overlays.Message_Overlays_C|GetProgressBar_Center _message_overlay_widget))
  (Widget|SetVisibility _progressbar_center "Visible")
  (Progress|SetPercent _progressbar_center 0.0) ; reset precentage
  (bind _returnvalue (Utilities|Time|SetTimerbyFunctionName 0 "Update Interaction Timer " 0.001 true))
  (Variables|Internal|SetInteraction%20Timer _returnvalue))

(fn AddtoInventory
  (params (Quantity :type Integer))
  (bind _char_ref (Variables|Internal|GetChar%20Ref))
  (bind _inventory_component (Variables|/Game/StarterInventory/FirstPerson/Blueprints/FirstPersonCharacter.FirstPersonCharacter_C|GetInventory%20Component _char_ref))
  (Variables|/Game/StarterInventory/Blueprints/Inventory.Inventory_C|SetInteraction%20Timer _inventory_component 0.0)
  (bind _item_array_location (Default|AddItemtoInventory _inventory_component self Quantity))
  (Audio|PlaySound2D (Variables|Default|GetPickup%20Sound))
  (return _item_array_location))

(fn CreateInteractionUI
  (params (Item%20Name :type Text) (Interaction%20verb :type Text))
  (Default|ResetInteractionTimer (Variables|/Game/StarterInventory/FirstPerson/Blueprints/FirstPersonCharacter.FirstPersonCharacter_C|GetInventory%20Component (Variables|Internal|GetChar%20Ref)))
  (bind _foundwidgets (Widget|GetAllWidgetsOfClass "/Game/StarterInventory/UMG/Message_Overlays.Message_Overlays_C" true))
  (for _array_element _foundwidgets
    (Widget|SetVisibility (Variables|/Game/StarterInventory/UMG/Message_Overlays.Message_Overlays_C|GetTextBlock_Middle _array_element) "Hidden") ; hide conflicting messages
  )
  (bind _returnvalue (UserInterface|CreateWidget "/Game/StarterInventory/UMG/Message_Overlays.Message_Overlays_C"))
  (bind _output_get (Variables|Internal|SetMessage%20Overlay%20Widget _returnvalue))
  (Widget|SetVisibility _output_get "Visible")
  (Variables|/Game/StarterInventory/UMG/Message_Overlays.Message_Overlays_C|SetMiddle%20Text%20 _output_get (Utilities|Text|FormatText "Hold \"{key}\" to {verb}
 {target name}" (Class|KismetInputLibrary|KeyGetDisplayName (.key (stale _array_element))) Interaction%20verb Item%20Name))
  (UserInterface|Viewport|AddtoViewport _output_get -1))

(fn RemoveInteractionUI
  (bind _message_overlay_widget (Variables|Internal|GetMessage%20Overlay%20Widget))
  (Utilities|IsValid _message_overlay_widget
    (:Is%20Valid
      (Widget|RemovefromParent _message_overlay_widget)
      ;[1 1 1] Extra protection to ensure removal and that none got stuck on screen
      (bind _foundwidgets (Widget|GetAllWidgetsOfClass "/Game/StarterInventory/UMG/Message_Overlays.Message_Overlays_C" true))
      (for _array_element _foundwidgets
        (Widget|RemovefromParent _array_element)))))

(fn UpdateInteractionTimer
  (bind _pickuptime (Variables|Default|GetPickupTime))
  (bind _char_ref (Variables|Internal|GetChar%20Ref))
  (bind _interaction_timer (Variables|Internal|GetInteraction%20Timer))
  (bind _message_overlay_widget (Variables|Internal|GetMessage%20Overlay%20Widget))
  (bind _inventory_component (Variables|/Game/StarterInventory/FirstPerson/Blueprints/FirstPersonCharacter.FirstPersonCharacter_C|GetInventory%20Component _char_ref))
  (bind _progressbar_center (Variables|/Game/StarterInventory/UMG/Message_Overlays.Message_Overlays_C|GetProgressBar_Center _message_overlay_widget))
  (bind _interaction_timer_2 (Variables|/Game/StarterInventory/Blueprints/Inventory.Inventory_C|GetInteraction%20Timer _inventory_component))
  (bind _returnvalue (Math|Float|Clamp(Float) _interaction_timer_2 0.0 _pickuptime))
  (if (Variables|/Game/StarterInventory/Blueprints/Inventory.Inventory_C|GetInteraction%20Button%20Pressed _inventory_component)
    (Progress|SetPercent _progressbar_center (/ _returnvalue _pickuptime))
    (if (>= _returnvalue _pickuptime)
      (Utilities|Time|ClearandInvalidateTimerbyHandle _interaction_timer)
      (CallFunction|AddtoInventory 1)
      ;[1 1 1] remove progress bar visual when complete but inventory is full
      (if (>= (Variables|/Script/UMG.ProgressBar|GetPercent _progressbar_center) 1.0)
        (Progress|SetPercent _progressbar_center 0.0)
        (Widget|SetVisibility _progressbar_center "Hidden")))
    (else
      (Utilities|Time|ClearandInvalidateTimerbyHandle _interaction_timer)
      (Widget|SetVisibility _progressbar_center "Hidden"))))

(fn CheckifItemOverlapIsCleared
  (bind _inventory_ref (Variables|Default|GetInventory%20ref))
  (bind _char_ref (Variables|/Game/StarterInventory/Blueprints/Inventory.Inventory_C|GetChar_ref _inventory_ref))
  (bind _inventory_component (Variables|/Game/StarterInventory/FirstPerson/Blueprints/FirstPersonCharacter.FirstPersonCharacter_C|GetInventory%20Component _char_ref))
  (Utilities|IsValid (Variables|/Game/StarterInventory/Blueprints/Inventory.Inventory_C|GetItem%20in%20Range _inventory_ref)
    (:Is%20Not%20Valid
      (Variables|/Game/StarterInventory/Blueprints/Inventory.Inventory_C|SetItem%20in%20Range _inventory_ref self)
      (CallFunction|CreateInteractionUI (Utilities|Text|ToText(String) (Variables|Default|GetItem%20Name)) (Variables|Default|GetInteraction%20verb))
      (if (Variables|/Game/StarterInventory/Blueprints/Inventory.Inventory_C|GetInteraction%20Button%20Pressed _inventory_component)
        (Variables|/Game/StarterInventory/Blueprints/Inventory.Inventory_C|SetInteraction%20Timer _inventory_component 0.0)
        (CallFunction|Interact)))))

(fn DismantleAction
  (params (Array%20Index :type Integer))
  (Development|PrintString "Dismantle from Item Base"))

(fn UseAction
  (Development|PrintString "Use from Item Base"))

(fn EquipAction
  (Development|PrintString "Equip from Item Base"))

(fn SetInventoryReffromPlayer
  (bind _asfirst_person_character (Utilities|Casting|CastToFirstPersonCharacter (Game|GetPlayerCharacter 0)))
  (Variables|Internal|SetChar%20Ref _asfirst_person_character)
  (Variables|Default|SetInventory%20ref (Variables|/Game/StarterInventory/FirstPerson/Blueprints/FirstPersonCharacter.FirstPersonCharacter_C|GetInventory%20Component _asfirst_person_character))
  (return))