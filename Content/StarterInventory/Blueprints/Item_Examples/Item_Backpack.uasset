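; Backpack item example for the starter inventory system that enlarges the player's inventory capacity.
; Its EquipAction event, the item's unique action, casts player character 0 to FirstPersonCharacter and adds ten to the InventoryComponent's maximum item count.
; It then refreshes the inventory UI list; the file shows no logic to undo the increase.
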(event EventBeginPlay
  (|CallParentFunction) ; This node is disabled and will not be called.\nDrag off pins to build functionality.
)

(event Collision|EventActorBeginOverlap
  (params (OtherActor :type Actor%20Object%20Reference))
  (|CallParentFunction OtherActor) ; This node is disabled and will not be called.\nDrag off pins to build functionality.
)

(event EventTick
  (params (DeltaSeconds :type Float%20%28single-precision%29)))

(event EventEquipAction
  ;[1 1 1] This is the Items unique action
  (bind _asfirst_person_character (Utilities|Casting|CastToFirstPersonCharacter (Game|GetPlayerCharacter 0)))
  (Variables|/Game/StarterInventory/Blueprints/Inventory.Inventory_C|SetInventory%20Item%20Max (Variables|/Game/StarterInventory/FirstPerson/Blueprints/FirstPersonCharacter.FirstPersonCharacter_C|GetInventory%20Component _asfirst_person_character) (+ (Variables|/Game/StarterInventory/Blueprints/Inventory.Inventory_C|GetInventory%20Item%20Max (Variables|/Game/StarterInventory/FirstPerson/Blueprints/FirstPersonCharacter.FirstPersonCharacter_C|GetInventory%20Component _asfirst_person_character)) 10))
  (Default|RefreshInventoryUIList (Variables|/Game/StarterInventory/FirstPerson/Blueprints/FirstPersonCharacter.FirstPersonCharacter_C|GetInventory%20Component _asfirst_person_character)))

(fn ConstructionScript
  (|CallParentFunction))