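; Crystal item for the starter inventory system, with a unique dismantle action that yields 25 Crystal Shards for the player.
; When the inventory is at its item limit, the player's InventoryComponent fills matching shard stacks and spawns the remainder.
; Otherwise it spawns a temporary shard actor at the world origin to add to the inventory, then refreshes the UI list and calls SplitUpStack.
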(event EventBeginPlay
  (|CallParentFunction) ; This node is disabled and will not be called.\nDrag off pins to build functionality.
)

(event Collision|EventActorBeginOverlap
  (params (OtherActor :type Actor%20Object%20Reference))
  (|CallParentFunction OtherActor) ; This node is disabled and will not be called.\nDrag off pins to build functionality.
)

(event EventDismantleAction
  (params (Array%20Index :type Integer))
  ;[1 1 1] Unique Crystal Action
  (bind _asfirst_person_character (Utilities|Casting|CastToFirstPersonCharacter (Game|GetPlayerCharacter 0)))
  (if (>= (Utilities|Array|Length (Variables|/Game/StarterInventory/Blueprints/Inventory.Inventory_C|GetInventory%20Array (Variables|/Game/StarterInventory/FirstPerson/Blueprints/FirstPersonCharacter.FirstPersonCharacter_C|GetInventory%20Component _asfirst_person_character))) (Variables|/Game/StarterInventory/Blueprints/Inventory.Inventory_C|GetInventory%20Item%20Max (Variables|/Game/StarterInventory/FirstPerson/Blueprints/FirstPersonCharacter.FirstPersonCharacter_C|GetInventory%20Component _asfirst_person_character))) ; Check if we are at our limit
    (Default|FillStacksandSpawnRemainder (Variables|/Game/StarterInventory/FirstPerson/Blueprints/FirstPersonCharacter.FirstPersonCharacter_C|GetInventory%20Component _asfirst_person_character) 25 "Crystal Shards" "/Game/StarterInventory/Blueprints/Item_Examples/Item_Crystal_Shards.Item_Crystal_Shards_C")
    (else
      (bind _returnvalue (Game|SpawnActorfromClass "/Game/StarterInventory/Blueprints/Item_Examples/Item_Crystal_Shards.Item_Crystal_Shards_C" (Math|Transform|MakeTransform "0, 0, 0") "Undefined" 0 0)) ; need to make a temp object so we can use it for item addition
      (Default|AddtoInventory _returnvalue 25)
      (Default|RefreshInventoryUIList (Variables|/Game/StarterInventory/FirstPerson/Blueprints/FirstPersonCharacter.FirstPersonCharacter_C|GetInventory%20Component _asfirst_person_character))
      (Default|SplitUpStack (Variables|/Game/StarterInventory/FirstPerson/Blueprints/FirstPersonCharacter.FirstPersonCharacter_C|GetInventory%20Component _asfirst_person_character)))))

(event EventTick
  (params (DeltaSeconds :type Float%20%28single-precision%29)))

(fn ConstructionScript
  (|CallParentFunction))