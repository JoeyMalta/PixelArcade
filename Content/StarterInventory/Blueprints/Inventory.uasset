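; Player inventory for the farmer character, handling item stacking, dropping, use, equip, dismantle and interaction input.
; Items live in a struct array: adds fill or create stacks, and overflow spawns on the ground ahead.
; Changes rebuild the open inventory widget, while world spawns and pickup destruction go through the character's replicated calls.
; Use, equip and dismantle spawn a hidden temporary item to run its class action, then destroy it on a timer.
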(event EventBeginPlay
  (bind _aspixel_farm_farmer (Utilities|Casting|CastToPixelFarm_Farmer (Game|GetPlayerCharacter 0)))
  (Variables|Default|SetChar_ref _aspixel_farm_farmer))

(fn CreateInventoryUI
  (Audio|PlaySound2D "/Engine/VREditor/Sounds/UI/Camera_Shutter.Camera_Shutter" 1.0 1.0 0.0 0 0)
  (Variables|Default|SetInventory%20Open true)
  (Variables|/Script/Engine.PlayerController|SetbShowMouseCursor (Game|GetPlayerController 0) true)
  (CallFunction|PurgeItemsfromStack) ; this will spawn objects on the ground if they got left in a stack that they no longer fit in
  (UI|RefreshInventoryUIList))

(fn RemoveInventoryUI
  (bind _returnvalue (Game|GetPlayerController 0))
  (Audio|PlaySound2D "/Engine/VREditor/Sounds/UI/Click_on_Button.Click_on_Button" 1.0 1.0 0.0 0 0)
  (Widget|RemovefromParent (Variables|Default|GetInventory%20Screen))
  (Variables|/Script/Engine.PlayerController|SetbShowMouseCursor _returnvalue false)
  (Variables|Default|SetInventory%20Open false)
  (Input|SetInputModeGameOnly _returnvalue))

(fn AddItemtoInventory
  (params (Item :type Item%20Base%20Object%20Reference) (Quantity :type Integer))
  (bind _stack_limit (Variables|/Game/StarterInventory/Blueprints/Item_Base.Item_Base_C|GetStack%20Limit Item))
  (bind _returnvalue (> _stack_limit 1))
  ;[1 1 1] Check if there is exsisting room in inventory And send to stack matching
  (Utilities|ResetMatchingVariables
    (:Output
      (if (.ReturnValue (Utilities|IsInventoryFulll?)) ; Check for Room for new items
        (if _returnvalue ; is it stackable?
          ;[1 1 1] Try to find a location in the array for a matching class item
          (bind _array_element (Utilities|Array|ForEachLoopwithBreak (Variables|Default|GetInventory%20Array) :!label _label)
            (:LoopBody
              (if (== (Utilities|GetClass Item) (.itemclass _array_element)) ; found matching class
                (if (Utilities|Enum|Equal(Enum) (.itemname _array_element) (Variables|/Game/StarterInventory/Blueprints/Item_Base.Item_Base_C|GetItem%20Name Item)) ; check for matching name
                  (if (> (.stacklimit _array_element) 1) ; is that match stackable?
                    (Variables|Default|SetMatch%20Found true)
                    (goto _label Break)))))
            (:Completed
              (if (Variables|Default|GetMatch%20Found) ; Check if a match was found
                ;[1 1 1] check for room in a matching stack
                (bind (_array_element_2 _array_index) (Utilities|Array|ForEachLoopwithBreak (Variables|Default|GetInventory%20Array) :!label _label_2)
                  (:LoopBody
                    (if (== (.itemclass _array_element_2) (Utilities|GetClass Item)) ; find matching class
                      (if (Utilities|Enum|Equal(Enum) (Variables|/Game/StarterInventory/Blueprints/Item_Base.Item_Base_C|GetItem%20Name Item) (.itemname _array_element_2)) ; check matching name
                        (if (< (.quantity _array_element_2) (.stacklimit _array_element_2)) ; Room in stack
                          (Variables|Default|SetStack%20Room%20Match true)
                          (Utilities|Array|SetArrayElem (Variables|Default|GetInventory%20Array) _array_index (Utilities|Struct|MakeInventory_Struct (.item _array_element_2) (+ (.quantity _array_element_2) Quantity) (.itemname _array_element_2) (.itemclass _array_element_2) (.stacklimit _array_element_2) (.image _array_element_2) (.interactiontypes _array_element_2) (.pickuptime _array_element_2))) ; Set updated Quantity info at matched index
                          (Default|DestroyItemReplicated (Variables|Default|GetChar_ref) Item)
                          (UI|RefreshInventoryUIList)
                          (CallFunction|CreateItemAddedMessage (Utilities|Text|ToText(String) (.itemname _array_element_2)) (.image _array_element_2))
                          (CallFunction|SplitUpStack)
                          (goto _label_2 Break)))))
                  (:Completed
                    ;[1 1 1] If no matches were found, try to make a new stack
                    (if (not (Variables|Default|GetStack%20Room%20Match)) ; no stack room was found, so lets make a new stack
                      (if (.ReturnValue (Utilities|IsInventoryFulll?)) ; Only allow a new stack if there is an empty slot
                        (bind (_added_inventory_index _added_item_name _image) (Utilities|AddNewItemWithoutStackAttempt Item Quantity) ; no matches so just add a new one
                          (:Output
                            (UI|RefreshInventoryUIList)
                            (CallFunction|CreateItemAddedMessage _added_item_name _image)
                            (CallFunction|SplitUpStack)
                            (Default|DestroyItemReplicated (Variables|Default|GetChar_ref) Item)
                            (return (Variables|Default|GetItem%20added%20Location))))
                        (else
                          (CallFunction|CreateInventoryFullMessage))))))
                (else
                  ;[1 1 1] if no exsisting match was found make a new entry
                  (bind _added_inventory_index_2 (Utilities|AddNewItemWithoutStackAttempt Item Quantity) ; no matches so just add a new one
                    (:Output
                      (UI|RefreshInventoryUIList) ; add the visuals to the inventory screen
                      (CallFunction|CreateItemAddedMessage (Utilities|Text|ToText(String) (.itemname (Utilities|Array|Get(acopy) (Variables|Default|GetInventory%20Array) _added_inventory_index_2))) (.image (Utilities|Array|Get(acopy) (Variables|Default|GetInventory%20Array) _added_inventory_index_2)))
                      (CallFunction|SplitUpStack)
                      (Default|DestroyItemReplicated (Variables|Default|GetChar_ref) Item)
                      (return (Variables|Default|GetItem%20added%20Location))))))))
          (else
            ;[1 1 1] if there is room and the item is not stackable make a new entry
            (bind (_added_inventory_index_3 _added_item_name_2 _image_2) (Utilities|AddNewItemWithoutStackAttempt Item Quantity)
              (:Output
                (UI|RefreshInventoryUIList)
                (CallFunction|CreateItemAddedMessage _added_item_name_2 _image_2)
                (CallFunction|SplitUpStack)
                (Default|DestroyItemReplicated (Variables|Default|GetChar_ref) Item)
                (return (Variables|Default|GetItem%20added%20Location))))))
        (elif _returnvalue ; Is it stackable?
          (goto _label_2)
          (else
            (CallFunction|CreateInventoryFullMessage) ; Tell the player the inventory is full
          ))))))

(fn RefreshInventoryUIList
  (if (Variables|Default|GetInventory%20Open)
    (Utilities|IsValid (Variables|Default|GetInventory%20Screen)
      (:Is%20Valid
        (Widget|RemovefromParent (Variables|Default|GetInventory%20Screen)))
      (:Is%20Not%20Valid
        _))
    (bind _returnvalue (UserInterface|CreateWidget "/Game/StarterInventory/UMG/Inventory_Screen.Inventory_Screen_C"))
    (Variables|/Game/StarterInventory/UMG/Inventory_Screen.Inventory_Screen_C|SetChar%20ref _returnvalue (Variables|Default|GetChar_ref))
    (bind _output_get (Variables|Default|SetInventory%20Screen _returnvalue))
    (UserInterface|Viewport|AddtoViewport _output_get 0)
    (for (_array_element _array_index) (Variables|Default|GetInventory%20Array)
      (bind _returnvalue_2 (UserInterface|CreateWidget "/Game/StarterInventory/UMG/Inventory_List_Item.Inventory_List_Item_C" (Game|GetPlayerController 0)))
      (Variables|/Game/StarterInventory/UMG/Inventory_List_Item.Inventory_List_Item_C|SetItem%20base%20Ref _returnvalue_2 (.item _array_element))
      (Variables|/Game/StarterInventory/UMG/Inventory_List_Item.Inventory_List_Item_C|Setparent _returnvalue_2 _output_get)
      (Variables|/Game/StarterInventory/UMG/Inventory_List_Item.Inventory_List_Item_C|SetItem%20Name _returnvalue_2 (Utilities|Text|ToText(String) (.itemname _array_element)))
      (Variables|/Game/StarterInventory/UMG/Inventory_List_Item.Inventory_List_Item_C|SetItem%20Quantity _returnvalue_2 (Utilities|Text|ToText(Integer) (.quantity _array_element)))
      (Variables|/Game/StarterInventory/UMG/Inventory_List_Item.Inventory_List_Item_C|SetInventory%20Array%20Position _returnvalue_2 _array_index)
      (Variables|/Game/StarterInventory/UMG/Inventory_List_Item.Inventory_List_Item_C|SetIcon_texture _returnvalue_2 (.image _array_element))
      (Widget|Panel|AddChild (Variables|/Game/StarterInventory/UMG/Inventory_Screen.Inventory_Screen_C|GetScrollBox_InventoryItems (Variables|Default|GetInventory%20Screen)) _returnvalue_2))))

(fn DropItem
  (params (Item%20ref :type Item%20Base%20Object%20Reference) (Item%20Array%20Position :type Integer) (Drop%20Quantity :type Integer))
  (Development|PrintString (Utilities|String|ToString(Integer) Drop%20Quantity))
  (CallFunction|SpawnItemsfromInventory (.itemclass (Utilities|Array|Get(acopy) (Variables|Default|GetInventory%20Array) Item%20Array%20Position)) Drop%20Quantity Item%20Array%20Position)
  (Utilities|DecrementItemfromStack Item%20Array%20Position Drop%20Quantity))

(fn UseItem
  (params (Item%20array%20location :type Integer))
  (bind _item_base_class (Utilities|DecrementItemfromStack Item%20array%20location 1)
    (:Output
      (bind _item_base_ref (CallFunction|CreateItemBase _item_base_class))
      ;[1 1 1] call function in item_base
      (Default|UseAction _item_base_ref))))

(fn DismantleItem
  (params (Item%20Array%20Position :type Integer))
  (bind _item_base_class (Utilities|DecrementItemfromStack Item%20Array%20Position 1)
    (:Output
      (bind _item_base_ref (CallFunction|CreateItemBase _item_base_class))
      ;[1 1 1] call function from item-Base class
      (Default|DismantleAction _item_base_ref))))

(fn CreateItemAddedMessage
  (params (Item%20Name :type Text) (ImageAsset :type Texture%202D%20Object%20Reference))
  (bind _foundwidgets (Widget|GetAllWidgetsOfClass "/Game/StarterInventory/UMG/Message_Overlays.Message_Overlays_C" true))
  (for _array_element _foundwidgets
    (Widget|SetVisibility (Variables|/Game/StarterInventory/UMG/Message_Overlays.Message_Overlays_C|GetTextBlock_Top _array_element) "Hidden"))
  (bind _returnvalue (UserInterface|CreateWidget "/Game/StarterInventory/UMG/Message_Overlays.Message_Overlays_C" (Game|GetPlayerController 0)))
  (Variables|/Game/StarterInventory/UMG/Message_Overlays.Message_Overlays_C|SetTop%20Text _returnvalue (Utilities|Text|FormatText "Added {name} to Inventory" Item%20Name))
  (Variables|/Game/StarterInventory/UMG/Message_Overlays.Message_Overlays_C|SetImage _returnvalue ImageAsset)
  (Widget|SetVisibility (Variables|/Game/StarterInventory/UMG/Message_Overlays.Message_Overlays_C|GetTextBlock_Top _returnvalue) "Visible")
  (UserInterface|Viewport|AddtoViewport _returnvalue 0)
  (Default|ShortDuration _returnvalue)
  (Audio|PlaySound2D "/Engine/VREditor/Sounds/UI/Click_on_Button_Cue.Click_on_Button_Cue" 1.0 1.0 0.0 0 0))

(fn EquipItem
  (params (Item%20array%20location :type Integer))
  (bind _item_base_class (Utilities|DecrementItemfromStack Item%20array%20location 1)
    (:Output
      (bind _item_base_ref (CallFunction|CreateItemBase _item_base_class))
      ;[1 1 1] cal function in item_base
      (Default|EquipAction _item_base_ref))))

(fn CreateInventoryFullMessage
  (bind _foundwidgets (Widget|GetAllWidgetsOfClass "/Game/StarterInventory/UMG/Message_Overlays.Message_Overlays_C" true))
  (for _array_element _foundwidgets
    (Widget|SetVisibility (Variables|/Game/StarterInventory/UMG/Message_Overlays.Message_Overlays_C|GetTextBlock_Top _array_element) "Hidden"))
  (bind _returnvalue (UserInterface|CreateWidget "/Game/StarterInventory/UMG/Message_Overlays.Message_Overlays_C" (Game|GetPlayerController 0)))
  (Variables|/Game/StarterInventory/UMG/Message_Overlays.Message_Overlays_C|SetTop%20Text _returnvalue (Utilities|Text|FormatText "Inventory Is Full"))
  (Widget|SetVisibility (Variables|/Game/StarterInventory/UMG/Message_Overlays.Message_Overlays_C|GetTextBlock_Top _returnvalue) "Visible")
  (UserInterface|Viewport|AddtoViewport _returnvalue 0)
  (Default|ShortDuration _returnvalue)
  (Audio|PlaySound2D "/Engine/EditorSounds/Notifications/CompileFailed.CompileFailed" 1.0 1.0 0.0 0 0))

(fn SplitUpStack
  (bind _inventory_array (Variables|Default|GetInventory%20Array))
  (for (_array_element _array_index) (Variables|Default|GetInventory%20Array)
    (if (> (.quantity _array_element) (.stacklimit _array_element))
      (Development|PrintString (Utilities|String|ToString(Text) (Utilities|Text|FormatText "Overage by: {index}" (Math|Integer|Absolute(Integer) (- (.stacklimit _array_element) (.quantity _array_element))))) false false)
      (bind _output_get (LocalVariables|SetStack%20Overage (Math|Integer|Absolute(Integer) (- (.stacklimit _array_element) (.quantity _array_element)))))
      (Utilities|Array|SetArrayElem _inventory_array _array_index (Utilities|Struct|MakeInventory_Struct (.item _array_element) (- (.quantity _array_element) _output_get) (.itemname _array_element) (.itemclass _array_element) (.stacklimit _array_element) (.image _array_element) (.interactiontypes _array_element) (.pickuptime _array_element))) ; reduce the original down to the stack limit
      (if (>= (Utilities|Array|Length (Variables|Default|GetInventory%20Array)) (Variables|Default|GetInventory%20Item%20Max)) ; if the inventory is full, spawn the remainder on the ground
        (CallFunction|SpawnItemsfromInventory (.itemclass _array_element) (LocalVariables|GetStack%20Overage) _array_index)
        (UI|RefreshInventoryUIList)
        (else
          (Utilities|Array|Add _inventory_array (Utilities|Struct|MakeInventory_Struct (.item _array_element) (LocalVariables|GetStack%20Overage) (.itemname _array_element) (.itemclass _array_element) (.stacklimit _array_element) (.image _array_element) (.interactiontypes _array_element) (.pickuptime _array_element))) ; if there is room, create a new stack
          (UI|RefreshInventoryUIList))))))

(fn CreateItemBase
  (params (Item%20Class :type Item%20Base%20Class%20Reference))
  ;[1 1 1] Spawn the actor so we can call its specific class functions
  (bind _returnvalue (Game|SpawnActorfromClass Item%20Class (Math|Transform|MakeTransform "0, 0, 0") "Undefined" 0 (Game|GetPlayerCharacter 0)))
  (bind _output_get (LocalVariables|SetItem%20Spawned _returnvalue))
  (Utilities|Array|Add (Variables|Default|GetTemp%20Item%20Spawn%20Array) _output_get)
  (Physics|SetSimulatePhysics (Variables|/Game/StarterInventory/Blueprints/Item_Base.Item_Base_C|GetStaticMesh _output_get) false)
  (Rendering|SetActorHiddenInGame _output_get true)
  (Utilities|Time|SetTimerbyFunctionName 0 "Clean Up" 1.0) ; this will delete the spawned items after use
  (return _output_get))

(fn CleanUp
  (bind _temp_item_spawn_array (Variables|Default|GetTemp%20Item%20Spawn%20Array))
  ;[1 1 1] Clean up all temp spawns
  (for _array_element _temp_item_spawn_array
    (Actor|DestroyActor _array_element))
  (Utilities|Array|Clear _temp_item_spawn_array))

(fn PurgeItemsfromStack
  (bind _inventory_array (Variables|Default|GetInventory%20Array))
  (bind _returnvalue (Utilities|Array|LastIndex _inventory_array))
  (bind _output (Utilities|Array|Get(acopy) _inventory_array _returnvalue))
  (if (> (Utilities|Array|Length _inventory_array) (Variables|Default|GetInventory%20Item%20Max))
    (CallFunction|SpawnItemsfromInventory (.itemclass _output) (.quantity _output) _returnvalue)
    (Utilities|Array|RemoveIndex _inventory_array _returnvalue)))

(fn SpawnItemsfromInventory
  (params (Class :type Item%20Base%20Object%20Reference) (Quantity%20to%20Spawn :type Integer) (Array%20Location :type Integer))
  (bind _returnvalue (Game|GetPlayerCharacter 0))
  (bind _inventory_array (Variables|Default|GetInventory%20Array))
  (bind _returnvalue_2 (Transformation|GetActorForwardVector _returnvalue))
  (bind _returnvalue_3 (Transformation|GetActorLocation _returnvalue))
  (bind _output (Utilities|Array|Get(acopy) _inventory_array Array%20Location))
  (bind _returnvalue_4 (* _returnvalue_2 2e+02))
  (bind _returnvalue_5 (+ _returnvalue_3 _returnvalue_4))
  (for _index (range 1 Quantity%20to%20Spawn)
    (bind _outhit (Collision|LineTraceByChannel (Math|Vector|MakeVector (.x _returnvalue_5) (.y _returnvalue_5) (.z _returnvalue_5)) (Math|Vector|MakeVector (.x _returnvalue_5) (.y _returnvalue_5) -3e+02) "TraceTypeQuery1" true 0 "None")) ; find a position  in front of the player and on the ground
    (Default|SpawnItemReplicated (Variables|Default|GetChar_ref) Class (Math|Conversions|ToTransform(Vector) (.location _outhit)) (.itemname _output) (.stacklimit _output) (.image _output) (.interactiontypes _output) (.pickuptime _output) false))
  (UI|RefreshInventoryUIList)
  (Audio|CreateSound2D "/Engine/VREditor/Sounds/UI/Click_on_Button_Cue.Click_on_Button_Cue" 1.0 1.0 0.0 0))

(fn FillStacksandSpawnRemainder
  (params (Quantity%20to%20Place :type Integer) (Item%20Name%20to%20Match :type String) (Class :type Item%20Base%20Class%20Reference))
  (LocalVariables|SetRemaining%20Quantity Quantity%20to%20Place)
  (for (_array_element _array_index) (Variables|Default|GetInventory%20Array)
    (if (or (== (.itemclass _array_element) Class) (Utilities|Enum|Equal(Enum) Item%20Name%20to%20Match (.itemname _array_element))) ; if it is a match
      (if (< (.quantity _array_element) (.stacklimit _array_element)) ; and if there is some room
        (LocalVariables|SetRemaining%20Quantity (- (LocalVariables|GetRemaining%20Quantity) (- (.stacklimit _array_element) (.quantity _array_element))))
        (Utilities|Array|SetArrayElem (Variables|Default|GetInventory%20Array) _array_index (Utilities|Struct|MakeInventory_Struct (.item _array_element) (+ (- (.stacklimit _array_element) (.quantity _array_element)) (.quantity _array_element)) (.itemname _array_element) (.itemclass _array_element) (.stacklimit _array_element) (.image _array_element) (.interactiontypes _array_element) (.pickuptime _array_element))))))
  (Development|PrintString (Utilities|String|ToString(Text) (Utilities|Text|FormatText "finished scan with {index} remaining" (LocalVariables|GetRemaining%20Quantity)))) ; spawn the remaining items into the world
  (CallFunction|SpawnItemsfromInventory Class (LocalVariables|GetRemaining%20Quantity) -1) ; set -1 to ignore array
)

(fn IncrementInteractionTImer
  (params (Delta :type Float%20%28single-precision%29))
  (if (Variables|Default|GetInteraction%20Button%20Pressed)
    (Utilities|IsValid (Variables|Default|GetItem%20in%20Range)
      (:Is%20Valid
        (Variables|Default|SetInteraction%20Timer (+ Delta (Variables|Default|GetInteraction%20Timer)))))))

(fn InventoryInputPressed
  (if (Variables|Default|GetInventory%20Open)
    (UI|RemoveInventoryUI)
    (else
      (UI|CreateInventoryUI))))

(fn InteractionInputPressed
  (bind _item_in_range (Variables|Default|GetItem%20in%20Range))
  (Variables|Default|SetInteraction%20Button%20Pressed true)
  (Utilities|IsValid _item_in_range ; if its a valid item_base start interaction
    (:Is%20Valid
      (Default|Interact _item_in_range))))

(fn InteractionInputReleased
  (Variables|Default|SetInteraction%20Button%20Pressed false)
  (Variables|Default|SetInteraction%20Timer 0.0))

(fn ResetInteractionTimer
  (Variables|Default|SetInteraction%20Timer 0.0))